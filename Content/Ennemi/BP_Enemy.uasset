(event OnComponentBeginOverlap(Sphere)
  (params (OverlappedComponent :type Primitive%20Component%20Object%20Reference) (OtherActor :type Actor%20Object%20Reference) (OtherComp :type Primitive%20Component%20Object%20Reference) (OtherBodyIndex :type Integer) (bFromSweep :type Boolean) (SweepResult :type Hit%20Result%20Structure%20%28by%20ref%29))
  (Utilities|Casting|CastToTopDownCharacter OtherActor)
  (Rendering|SetVisibility (Variables|Default|GetWidget) true false))

(event OnComponentEndOverlap(Sphere)
  (params (OverlappedComponent :type Primitive%20Component%20Object%20Reference) (OtherActor :type Actor%20Object%20Reference) (OtherComp :type Primitive%20Component%20Object%20Reference) (OtherBodyIndex :type Integer))
  (Utilities|Casting|CastToTopDownCharacter OtherActor)
  (Rendering|SetVisibility (Variables|Default|GetWidget) false false))

(event Custom|CustomEvent
  (bind _astop_down_character (Utilities|Casting|CastToTopDownCharacter (Game|GetPlayerCharacter 0)))
  (Variables|Default|SetCharacter%20Ref _astop_down_character)
  (bind _ashealth_widget (Utilities|Casting|CastToHealthWidget (UserInterface|GetUserWidgetObject (Variables|Default|GetWidget))))
  (bind _output_get (Variables|Default|SetAs%20Health%20Widget _ashealth_widget))
  (Variables|/Game/Ennemi/HealthWidget.HealthWidget_C|Sethealth _output_get 0.0))

(event EventBeginPlay)

(event EventTick
  (params (DeltaSeconds :type Float%20%28single-precision%29))
  (Development|PrintString (Utilities|String|Append "Enemy" (Utilities|String|ToString(Integer) (Variables|Default|GetHealth))) true true "(R=0.000000,G=0.660000,B=1.000000,A=1.000000)" 0.0))

(event Game|Damage|EventAnyDamage
  (params (Damage :type Float%20%28single-precision%29) (DamageType :type Damage%20Type%20Object%20Reference) (InstigatedBy :type Controller%20Object%20Reference) (DamageCauser :type Actor%20Object%20Reference))
  (bind _output_get (Variables|Default|SetHealth (Math|Float|Truncate (- (Variables|Default|GetHealth) Damage))))
  (Variables|/Game/Ennemi/HealthWidget.HealthWidget_C|Sethealth (Variables|Default|GetAs%20Health%20Widget) (Math|Conversions|ToFloat(Integer) _output_get))
  (if (<= _output_get 0)
    (Physics|SetSimulatePhysics (Variables|Character|GetMesh) true)
    (Collision|SetCollisionEnabled (Variables|Collision|GetCapsuleComponent) "NoCollision")
    (Class|Pawn|DetachfromControllerPendingDestroy)
    (Components|Animation|SetAnimationMode (Variables|Character|GetMesh) "AnimationBlueprint")))

(event Collision|EventActorBeginOverlap
  (params (OtherActor :type Actor%20Object%20Reference)))

(fn ConstructionScript)