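; AI controller for enemies that starts the BT_Enemy behavior tree on BeginPlay.
; AI Perception updates on a TopDownCharacter with health above zero write to the blackboard: a sensed character becomes PlayerRef.
; When sensing is lost, the stimulus location is saved as LastPlayerLocation and PlayerRef is cleared.
; A ResetPlayerRef event also clears PlayerRef on demand.
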(event OnTargetPerceptionUpdated(AIPerception)
  (params (Actor :type Actor%20Object%20Reference) (Stimulus :type AI%20Stimulus%20Structure))
  (bind _astop_down_character (Utilities|Casting|CastToTopDownCharacter Actor))
  (if (> (Variables|/Game/TopDownBP/Blueprints/TopDownCharacter.TopDownCharacter_C|GetHealth _astop_down_character) 0)
    (if (.bsuccessfullysensed Stimulus)
      (AI|Components|Blackboard|SetValueasObject (AI|GetBlackboard 0) (Utilities|String|StringToName "PlayerRef") _astop_down_character)
      (else
        (AI|Components|Blackboard|SetValueasVector (AI|GetBlackboard 0) (Utilities|String|StringToName "LastPlayerLocation") (.stimuluslocation Stimulus))
        (AI|Components|Blackboard|ClearValue (AI|GetBlackboard 0) (Utilities|String|StringToName "PlayerRef"))))))

(event Custom|ResetPlayerRef
  (AI|Components|Blackboard|ClearValue (AI|GetBlackboard 0) (Utilities|String|StringToName "PlayerRef")))

(event EventBeginPlay
  (AI|RunBehaviorTree "/Game/Ennemi/BT_Enemy.BT_Enemy"))

(event EventTick
  (params (DeltaSeconds :type Float%20%28single-precision%29)))

(fn ConstructionScript)